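; GM_Algorithm is a Blueprint that runs a stack-based summing exercise on BeginPlay and prints the result.
; It draws a random count K up to MaxK, then generates that many random numbers bounded by MaxNum.
; NumArray acts as a stack: a zero removes the last entry and any other value is appended.
; The remaining entries are summed, and both K and the sum are printed as debug strings.
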(event EventBeginPlay
  (bind _numarray (Variables|Default|GetNumArray))
  (bind _output_get (Variables|Default|SetK (Math|Random|RandomIntegerinRange 1 (Variables|Default|GetMaxK))))
  (Development|PrintString (Utilities|String|Append "K is" (Utilities|String|ToString(Integer) _output_get)))
  (for _index (range 1 (Variables|Default|GetK))
    (bind _output_get_2 (Variables|Default|SetTempNum (Class|KismetMathLibrary|RandomInteger64 (Variables|Default|GetMaxNum))))
    (if (== _output_get_2 0)
      (Utilities|Array|RemoveIndex _numarray (Utilities|Array|LastIndex _numarray))
      (else
        (Utilities|Array|Add (Variables|Default|GetNumArray) _output_get_2))))
  (for _array_element (Variables|Default|GetNumArray)
    (Variables|Default|SetSum (+ (Variables|Default|GetSum) _array_element)))
  (Development|PrintString (Utilities|String|Append "sum is" (Utilities|String|ToString(Integer) (Variables|Default|GetSum)))))

(fn ConstructionScript)